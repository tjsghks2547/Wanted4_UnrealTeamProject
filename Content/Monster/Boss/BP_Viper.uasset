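; BP_Viper is a boss monster Blueprint that handles the hit detection and damage for Viper's attacks.
; OnAttackCheckStart and OnAttackCheckEnd, noted as called from AnimNotify_EnemyAttackCheck, switch the AttackCollision component between query-only and no collision.
; Overlapping actors receive Damage with Viper as causer, and the HitActors list, cleared at each start, limits each actor to one hit per attack window.
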(event OnComponentBeginOverlap(AttackCollision)
  (params (OverlappedComponent :type Primitive%20Component%20Object%20Reference) (OtherActor :type Actor%20Object%20Reference) (OtherComp :type Primitive%20Component%20Object%20Reference) (OtherBodyIndex :type Integer) (bFromSweep :type Boolean) (SweepResult :type Hit%20Result%20Structure%20%28by%20ref%29))
  (bind _hitactors (Variables|Attack|GetHitActors))
  ;[0.15 0.15 0.15 0.5] 충돌처리 (AnimNotify_EnemyAttackCheck내에서 호출)
  (if (not (Utilities|Array|ContainsItem _hitactors OtherActor))
    (Utilities|Array|Add _hitactors OtherActor)
    (Game|Damage|ApplyDamage OtherActor (Variables|Attack|GetDamage) (Pawn|GetController) self)))

(event Custom|OnAttackCheckEnd
  ;[0.15 0.15 0.15 0.5] 충돌처리 (AnimNotify_EnemyAttackCheck내에서 호출)
  (Collision|SetCollisionEnabled (Variables|Attack|GetAttackCollision) "NoCollision"))

(event Custom|OnAttackCheckStart
  ;[0.15 0.15 0.15 0.5] 충돌처리 (AnimNotify_EnemyAttackCheck내에서 호출)
  (Utilities|Array|Clear (Variables|Attack|GetHitActors))
  (Collision|SetCollisionEnabled (Variables|Attack|GetAttackCollision) "QueryOnly"))

(event EventBeginPlay)

(event Collision|EventActorBeginOverlap
  (params (OtherActor :type Actor%20Object%20Reference)))

(event EventTick
  (params (DeltaSeconds :type Float%20%28single-precision%29)))

(fn ConstructionScript)