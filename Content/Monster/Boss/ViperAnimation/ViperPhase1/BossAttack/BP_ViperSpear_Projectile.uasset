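; Boomerang-style spear projectile for the Viper boss that flies out toward the player and returns.
; BeginPlay caches the player's position; Tick manually moves the spear horizontally at that target's height until MaxDistance, then tracks Viper back and destroys it nearby.
; Sphere overlaps damage the player using Viper's damage, with duplicate checks through Viper's HitActors, cleared after each player hit.
; Older player-homing, socket-return and ProjectileMovement logic remains disconnected.
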(event OnComponentBeginOverlap(Sphere)
  (params (OverlappedComponent :type Primitive%20Component%20Object%20Reference) (OtherActor :type Actor%20Object%20Reference) (OtherComp :type Primitive%20Component%20Object%20Reference) (OtherBodyIndex :type Integer) (bFromSweep :type Boolean) (SweepResult :type Hit%20Result%20Structure%20%28by%20ref%29))
  (bind _viper (Variables|Default|GetViper))
  (bind _hitactors (Variables|/Game/Monster/Boss/BP_Viper.BP_Viper_C|GetHitActors _viper))
  ;[0.15 0.15 0.15 0.5] 충돌 처리 및 대미지 적용
  (if (not (Utilities|Array|ContainsItem _hitactors OtherActor))
    (Utilities|Array|Add _hitactors OtherActor)
    (bind _asbp_kzcharacter_player (Utilities|Casting|CastToBP_KZCharacterPlayer OtherActor))
    (Class|KZCharacterPlayer|ProcessDamage _asbp_kzcharacter_player (Utilities|Struct|MakeDamageData (Variables|/Game/Monster/Boss/BP_Viper.BP_Viper_C|GetDamage _viper) _viper))
    (Utilities|Array|Clear _hitactors)))

(event EventBeginPlay
  (Utilities|FlowControl|Sequence
    (:then_0
      (bind _returnvalue (Actor|GetActorOfClass "/Game/Monster/Boss/BP_Viper.BP_Viper_C"))
      (Variables|Default|SetViper _returnvalue)
      ;[0.15 0.15 0.15 0.5] 스폰 위치 초기화
      (Variables|Default|SetSpawnLocation (Transformation|GetActorLocation))
      ;[0.15 0.15 0.15 0.5] 목적지 초기화
      (Variables|Default|SetTargetLocation (Transformation|GetActorLocation (Game|GetPlayerCharacter 0))))
    (:then_1
      (Variables|Default|SetbIsStarted true)
      (Transformation|SetActorRotation "0.000000,0.000000,90.000000"))))

(event Collision|EventActorBeginOverlap
  (params (OtherActor :type Actor%20Object%20Reference)))

(event EventTick
  (params (DeltaSeconds :type Float%20%28single-precision%29))
  (bind _returnvalue (Transformation|GetActorLocation))
  (bind _returnvalue_2 (Transformation|GetActorLocation))
  ;[0.15 0.15 0.15 0.5] 유도형 로직
  (Utilities|FlowControl|Sequence
    (:then_0
      (Utilities|IsValid (Variables|Default|GetViper)
        (:Is%20Valid
          (if (Variables|Default|GetIsReturning)
            (Variables|Default|SetTargetLocation (Transformation|GetActorLocation (Variables|Default|GetViper)))
            ;[0.15 0.15 0.15 0.5] return
            (Variables|Default|SetDirectionVector (Transformation|GetActorLocation))
            (Transformation|SetActorLocation (+ (Math|Vector|MakeVector (.x _returnvalue_2) (.y _returnvalue_2) (.z (Variables|Default|GetTargetLocation))) (* (Math|Vector|Normalize (Math|Vector|MakeVector (.X (Math|Vector|BreakVector (- (Variables|Default|GetTargetLocation) (Variables|Default|GetDirectionVector)))) (.Y (Math|Vector|BreakVector (- (Variables|Default|GetTargetLocation) (Variables|Default|GetDirectionVector)))) 0.0)) (Variables|Default|GetSpeed) DeltaSeconds)) false false)
            ;;[0.15 0.15 0.15 0.5] 리턴 상태 (회수)
            (if (< (Math|Vector|Distance(Vector) (Transformation|GetActorLocation) (Transformation|GetActorLocation (Variables|Default|GetViper))) 3e+02)
              (Actor|DestroyActor))
            (else
              ;;[0.15 0.15 0.15 0.5] 목적지 근처 도착 검사
              (if (>= (Math|Vector|Distance(Vector) (Variables|Default|GetSpawnLocation) (Transformation|GetActorLocation)) (Variables|Default|GetMaxDistance))
                (Variables|Default|SetIsReturning true)
                (Variables|Default|SetbIsStarted false)))))))
    (:then_1
      ;[0.15 0.15 0.15 0.5] forward
      (if (Variables|Default|GetbIsStarted)
        (Transformation|SetActorLocation (+ (Math|Vector|MakeVector (.x _returnvalue) (.y _returnvalue) (.z (Variables|Default|GetTargetLocation))) (* (Math|Vector|Normalize (Math|Vector|MakeVector (.X (Math|Vector|BreakVector (- (Variables|Default|GetTargetLocation) (Variables|Default|GetSpawnLocation)))) (.Y (Math|Vector|BreakVector (- (Variables|Default|GetTargetLocation) (Variables|Default|GetSpawnLocation)))) 0.0)) (Variables|Default|GetSpeed) DeltaSeconds)) false false)))))

(fn ConstructionScript)