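; Spear projectile for the Viper boss that flies toward the player's position captured at spawn, then returns to Viper and destroys itself.
; Tick moves it by boss phase: Normal Form flies straight to a max distance, while Enhance eases in with VInterpTo and waits on a timer before returning.
; Sphere overlaps damage the player, filtered through Viper's HitActors in Normal Form or starting a looping damage-over-time timer in Enhance.
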(event OnComponentBeginOverlap(Sphere)
  (params (OverlappedComponent :type Primitive%20Component%20Object%20Reference) (OtherActor :type Actor%20Object%20Reference) (OtherComp :type Primitive%20Component%20Object%20Reference) (OtherBodyIndex :type Integer) (bFromSweep :type Boolean) (SweepResult :type Hit%20Result%20Structure%20%28by%20ref%29))
  (bind _viper (Variables|Default|GetViper))
  (bind _hitactors (Variables|/Game/Monster/Boss/BP_Viper.BP_Viper_C|GetHitActors _viper))
  ;[0.15 0.15 0.15 0.5] 충돌 처리 및 대미지 적용
  (switch Utilities|FlowControl|Switch|SwitchonEBossPhase (Variables|Default|GetViperPhase)
    (:Phase1A
      ;;[0.15 0.15 0.15 0.5] 1페이즈 대미지 처리: forward시
      (if (not (Utilities|Array|ContainsItem _hitactors OtherActor))
        (Utilities|Array|Add _hitactors OtherActor)
        (bind _asbp_kzcharacter_player (Utilities|Casting|CastToBP_KZCharacterPlayer OtherActor))
        (Class|KZCharacterPlayer|ProcessDamage _asbp_kzcharacter_player (Utilities|Struct|MakeDamageData (Variables|/Game/Monster/Boss/BP_Viper.BP_Viper_C|GetDamage _viper) _viper 0.0 false))))
    (:Phase1B
      ;;[0.15 0.15 0.15 0.5] 1.5페이즈 대미지처리
      (Utilities|IsValid (Variables|Default|GetViper)
        (:Is%20Valid
          (bind _asbp_kzcharacter_player_2 (Utilities|Casting|CastToBP_KZCharacterPlayer OtherActor))
          (Variables|Default|SetOverlappedPlayer _asbp_kzcharacter_player_2)
          (Utilities|Time|SetTimerbyFunctionName 0 "ApplyTickDamage" 0.2 true))))))

(event Custom|TimeOut
  ;[0.15 0.15 0.15 0.5] 목적지 근처 도착 검사
  (Variables|Default|SetIsReturning true)
  (Variables|Default|SetbIsStarted false))

(event Custom|ApplyTickDamage
  (bind _viper (Variables|Default|GetViper))
  ;[0.15 0.15 0.15 0.5] 충돌 처리 및 대미지 적용
  ;;[0.15 0.15 0.15 0.5] 1.5페이즈 대미지처리
  (Utilities|IsValid (Variables|Default|GetViper)
    (:Is%20Valid
      (bind _asbp_kzcharacter_player (Utilities|Casting|CastToBP_KZCharacterPlayer (stale OnComponentBeginOverlap(Sphere) OtherActor)))
      (Variables|Default|SetOverlappedPlayer _asbp_kzcharacter_player)
      (Class|KZCharacterPlayer|ProcessDamage _asbp_kzcharacter_player (Utilities|Struct|MakeDamageData (Variables|/Game/Monster/Boss/BP_Viper.BP_Viper_C|GetDamage _viper) _viper 0.0 true)))))

(event EventBeginPlay
  (bind _returnvalue (Transformation|GetActorLocation))
  (bind _returnvalue_2 (Game|GetPlayerCharacter 0))
  (bind _returnvalue_3 (Transformation|GetActorLocation _returnvalue_2))
  (bind _returnvalue_4 (Math|Rotator|FindLookatRotation _returnvalue _returnvalue_3))
  (bind (_roll _pitch _yaw) (Math|Rotator|BreakRotator (Math|Rotator|MakeRotator 0.0 (.pitch _returnvalue_4) (.yaw _returnvalue_4))))
  (Utilities|FlowControl|Sequence
    (:then_0
      (bind _returnvalue_5 (Actor|GetActorOfClass "/Game/Monster/Boss/BP_Viper.BP_Viper_C"))
      (bind _output_get (Variables|Default|SetViper _returnvalue_5))
      (Variables|Default|SetViperPhase (Variables|/Script/Khazan.KZBossCharacter|GetCurrentPhase _output_get))
      ;[0.15 0.15 0.15 0.5] 리턴 위치 최기화
      (Variables|Default|SetReturnLocation (Transformation|GetActorLocation (Variables|Default|GetViper)))
      ;[0.15 0.15 0.15 0.5] 스폰 위치 초기화
      (Variables|Default|SetSpawnLocation (Transformation|GetActorLocation))
      ;[0.15 0.15 0.15 0.5] 목적지 초기화
      (Variables|Default|SetTargetLocation (Transformation|GetActorLocation (Game|GetPlayerCharacter 0))))
    (:then_1
      (Variables|Default|SetbIsStarted true)
      (if (Utilities|Enum|Equal(Enum) (Variables|/Script/Khazan.KZBossCharacter|GetCurrentPhase (Variables|Default|GetViper)) "Phase1A")
        (Transformation|SetActorRotation "0.000000,0.000000,90.000000")
        (else
          ;[0.15 0.15 0.15 0.5] 1.5페이즈 회전날 각도조절
          (Transformation|SetActorRotation (Math|Rotator|MakeRotator _roll _pitch _yaw))
          (Variables|Default|SetSpeed 15.0))))))

(event Collision|EventActorBeginOverlap
  (params (OtherActor :type Actor%20Object%20Reference)))

(event EventTick
  (params (DeltaSeconds :type Float%20%28single-precision%29))
  (bind _returnvalue (Transformation|GetActorLocation))
  (bind _returnvalue_2 (Transformation|GetActorLocation))
  (bind _viper (Variables|Default|GetViper))
  (bind _targetlocation (Variables|Default|GetTargetLocation))
  (bind _spawnlocation (Variables|Default|GetSpawnLocation))
  (bind _returnvalue_3 (- _targetlocation _spawnlocation))
  (bind (_x _y) (Math|Vector|BreakVector _returnvalue_3))
  (switch Utilities|FlowControl|Switch|SwitchonEBossPhase (Variables|Default|GetViperPhase)
    (:Phase1A
      ;[0.15 0.15 0.15 0.5] 직선형 로직
      (Utilities|FlowControl|Sequence
        (:then_0
          (Utilities|IsValid _viper
            (:Is%20Valid
              (if (Variables|Default|GetIsReturning)
                ;;[0.15 0.15 0.15 0.5] 1페이즈 대미지 처리: Return 대미지 처리를 위한 Return시 clear
                (Utilities|Array|Clear (Variables|/Game/Monster/Boss/BP_Viper.BP_Viper_C|GetHitActors _viper))
                ;;[0.15 0.15 0.15 0.5] return
                (Variables|Default|SetReturnLocation (Transformation|GetActorLocation (Variables|Default|GetViper)))
                (Variables|Default|SetDirectionVector (Transformation|GetActorLocation))
                (Transformation|SetActorLocation (+ (Math|Vector|MakeVector (.x _returnvalue_2) (.y _returnvalue_2) (.z (Variables|Default|GetReturnLocation))) (* (Math|Vector|Normalize (Math|Vector|MakeVector (.X (Math|Vector|BreakVector (- (Variables|Default|GetReturnLocation) (Variables|Default|GetDirectionVector)))) (.Y (Math|Vector|BreakVector (- (Variables|Default|GetReturnLocation) (Variables|Default|GetDirectionVector)))) 0.0)) (Variables|Default|GetSpeed) DeltaSeconds)) false false)
                (if (< (Math|Vector|Distance(Vector) (Transformation|GetActorLocation) (Transformation|GetActorLocation (Variables|Default|GetViper))) 3e+02)
                  (Actor|DestroyActor))
                (else
                  ;;[0.15 0.15 0.15 0.5] 목적지 근처 도착 검사
                  (if (>= (Math|Vector|Distance(Vector) (Variables|Default|GetSpawnLocation) (Transformation|GetActorLocation)) (Variables|Default|GetMaxDistance))
                    (Variables|Default|SetIsReturning true)
                    (Variables|Default|SetbIsStarted false)))))))
        (:then_1
          ;;[0.15 0.15 0.15 0.5] forward
          (if (Variables|Default|GetbIsStarted)
            (Transformation|SetActorLocation (+ (Math|Vector|MakeVector (.x _returnvalue) (.y _returnvalue) (.z (Variables|Default|GetTargetLocation))) (* (Math|Vector|Normalize (Math|Vector|MakeVector _x _y 0.0)) (Variables|Default|GetSpeed) DeltaSeconds)) false false)))))
    (:Phase1B
      (Utilities|FlowControl|Sequence
        (:then_0
          (Utilities|IsValid (Variables|Default|GetViper)
            (:Is%20Valid
              (if (Variables|Default|GetIsReturning)
                (Transformation|SetActorLocation (Math|Interpolation|VInterpTo (Transformation|GetActorLocation) (Transformation|GetActorLocation (Variables|Default|GetViper)) DeltaSeconds (Variables|Default|GetSpeed)) false false)
                (if (< (Math|Vector|Distance(Vector) (Transformation|GetActorLocation) (Transformation|GetActorLocation (Variables|Default|GetViper))) 3e+02)
                  (Actor|DestroyActor))
                (else
                  ;[0.15 0.15 0.15 0.5] 목적지 근처 도착 검사
                  (if (>= 1.5e+02 (Math|Vector|Distance(Vector) (Variables|Default|GetTargetLocation) (Transformation|GetActorLocation)))
                    (if (not (Variables|Default|GetbReached))
                      (Variables|Default|SetbReached true)
                      (Utilities|Time|SetTimerbyEvent (delegate Custom|TimeOut) (Variables|Default|GetFlightTime)))))))))
        (:then_1
          (if (not (Variables|Default|GetIsReturning))
            ;[0.15 0.15 0.15 0.5] Homing 상태 (유도)
            (Transformation|SetActorLocation (Math|Interpolation|VInterpTo (Transformation|GetActorLocation) (Variables|Default|GetTargetLocation) DeltaSeconds (Variables|Default|GetSpeed)) false false)))))))

(fn ConstructionScript)