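; BPC_PlatformRider is an actor component for BP_KZCharacterPlayer, apparently meant to handle riding on platforms.
; On BeginPlay it casts its owner to that class and caches the character and its movement component.
; While riding mode is on, Tick checks whether the movement component's current floor has a valid hit component.
; The logic is unfinished: nothing follows that check, and a velocity read is left unconnected.
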(event EventBeginPlay
  (bind _asbp_kzcharacter_player (Utilities|Casting|CastToBP_KZCharacterPlayer (Components|GetOwner)))
  (bind _output_get (Variables|Default|SetOwnderCharacter _asbp_kzcharacter_player))
  (Variables|Default|SetMovementComponent (Variables|/Script/Engine.Character|GetCharacterMovement _output_get)))

(event EventTick
  (params (DeltaSeconds :type Float%20%28single-precision%29))
  (if (Variables|Default|GetIsRidingMode)
    (if (Utilities|IsValid (.HitComponent (Collision|BreakHitResult (.HitResult (Utilities|Struct|BreakFindFloorResult (Variables|/Script/Engine.CharacterMovementComponent|GetCurrentFloor (Variables|Default|GetMovementComponent)))))))
      _)))