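; BP_SavePoint is a save point actor that persists the player's position in the "savepoint1" save slot.
; On BeginPlay it loads BP_SaveGame and moves the player to the stored position, or creates a save with the current position.
; When KZCharacterPlayer overlaps its Cube, it saves that character's location through the cached save object.
; That cache is only set when an existing save loads.
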(event OnComponentBeginOverlap(Cube)
  (params (OverlappedComponent :type Primitive%20Component%20Object%20Reference) (OtherActor :type Actor%20Object%20Reference) (OtherComp :type Primitive%20Component%20Object%20Reference) (OtherBodyIndex :type Integer) (bFromSweep :type Boolean) (SweepResult :type Hit%20Result%20Structure%20%28by%20ref%29))
  (bind _as_bp_save_game (Variables|Default|GetAs%20BP%20Save%20Game))
  (bind _askzcharacter_player (Utilities|Casting|CastToKZCharacterPlayer OtherActor))
  (Variables|/Game/Map/Actor/BP_SaveGame.BP_SaveGame_C|SetPlayerPos _as_bp_save_game (Transformation|GetActorLocation _askzcharacter_player))
  (SaveGame|SaveGametoSlot _as_bp_save_game "savepoint1"))

(event EventBeginPlay
  (bind _returnvalue (SaveGame|DoesSaveGameExist "savepoint1"))
  (if _returnvalue
    (bind _returnvalue_2 (SaveGame|LoadGamefromSlot "savepoint1"))
    (bind _asbp_save_game (Utilities|Casting|CastToBP_SaveGame _returnvalue_2))
    (Variables|Default|SetAs%20BP%20Save%20Game _asbp_save_game)
    (Transformation|SetActorLocation (Game|GetPlayerCharacter 0) (Variables|/Game/Map/Actor/BP_SaveGame.BP_SaveGame_C|GetPlayerPos _asbp_save_game) false false)
    (else
      (bind _returnvalue_3 (SaveGame|CreateSaveGameObject "/Game/Map/Actor/BP_SaveGame.BP_SaveGame_C"))
      (Variables|/Game/Map/Actor/BP_SaveGame.BP_SaveGame_C|SetPlayerPos _returnvalue_3 (Transformation|GetActorLocation (Game|GetPlayerCharacter 0)))
      (SaveGame|SaveGametoSlot _returnvalue_3 "savepoint1"))))

(event Collision|EventActorBeginOverlap
  (params (OtherActor :type Actor%20Object%20Reference)))

(event EventTick
  (params (DeltaSeconds :type Float%20%28single-precision%29)))

(fn ConstructionScript)