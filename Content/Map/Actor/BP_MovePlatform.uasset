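; BP_MovePlatform is a moving platform that travels along its Arrow's forward direction from its starting position.
; A timeline starts on BeginPlay at a configurable play rate, and its curve value times a distance sets the offset.
; Each update, player characters overlapping the Box whose movement mode is None are teleported by the platform's position delta, carrying them along manually.
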(event EventBeginPlay
  (bind _output_get (Variables|Default|Set최초위치 (Transformation|GetActorLocation)))
  (Variables|Default|SetPreviousLocation _output_get)
  (Components|Timeline|SetPlayRate (Variables|Default|Get이동그래프) (Variables|Default|Get재생속도))
  (bind _이동값 (Timeline|이동그래프 Play)
    (:Update
      (Transformation|SetActorLocation (+ (Variables|Default|Get최초위치) (* (Math|Vector|GetForwardVector (Variables|Default|GetArrow)) (* _이동값 (Variables|Default|Get이동거리)))) false false)
      (Utilities|FlowControl|Sequence
        (:then_0
          (Variables|Default|SetGapDist (- (Transformation|GetActorLocation) (Variables|Default|GetPreviousLocation))))
        (:then_1
          (for _array_element (Collision|GetOverlappingActors (Variables|Default|GetBox) "/Game/Khazan/Blueprint/BP_KZCharacterPlayer.BP_KZCharacterPlayer_C" :!class /Script/Engine.PrimitiveComponent)
            (bind _asbp_kzcharacter_player (Utilities|Casting|CastToBP_KZCharacterPlayer _array_element)
              (:then
                (if (Utilities|Enum|Equal(Enum) (Variables|/Script/Engine.CharacterMovementComponent|GetMovementMode (Variables|/Script/Engine.Character|GetCharacterMovement _asbp_kzcharacter_player)) "MOVE_None")
                  (Transformation|SetActorLocation _array_element (+ (Transformation|GetActorLocation _array_element) (Variables|Default|GetGapDist)) false true)))
              (:CastFailed
                (Development|PrintString "Hello")))))
        (:then_2
          (Variables|Default|SetPreviousLocation (Transformation|GetActorLocation)))))))

(event Collision|EventActorBeginOverlap
  (params (OtherActor :type Actor%20Object%20Reference)))

(fn ConstructionScript)